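; BP_MuzzleFlash is a muzzle flash actor with logic to turn it toward the player, caching the BP_Player reference on BeginPlay.
; FacingPlayer loops on a 0.2-second retriggerable delay, interpolating yaw toward the player's spring arm like a yaw-only billboard.
; The only call to FacingPlayer in this Blueprint is disconnected, so the actor does not start the loop itself.
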(event `self.ReceiveBeginPlay`
  (bind _asbp_player (cast `/Game/Char/Player/BP_Player` (`GameplayStatics.GetPlayerCharacter` 0)))
  (set `self.PlayerRef` _asbp_player))

(event `FacingPlayer`
  (bind (_returnvalue_roll _returnvalue_pitch _returnvalue_yaw) (`KismetMathLibrary.BreakRotator` (`KismetMathLibrary.RInterpTo` (`self.K2_GetActorRotation`) (`KismetMathLibrary.FindLookAtRotation` (`self.K2_GetActorLocation`) (`SceneComponent.K2_GetComponentLocation` (`/Game/Char/Player/BP_Player.SpringArm` (`self.PlayerRef`)))) (`GameplayStatics.GetWorldDeltaSeconds`) 150.0)))
  (`self.K2_SetActorRotation` (`KismetMathLibrary.MakeRotator` 0.0 0.0 _returnvalue_yaw) :!label _label)
  (`KismetSystemLibrary.RetriggerableDelay` 0.2)
  (goto _label))

(fn `UserConstructionScript`)
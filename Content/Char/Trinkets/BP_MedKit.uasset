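; BP_MedKit is a health pickup that heals the player on contact and then destroys itself.
; On BeginPlay it caches player 0's BP_Player and starts a retriggerable-delay loop that periodically interpolates its yaw to face that player.
; Overlapping the MedKitCollider adds a fixed amount of health, but only when that player is below max health, so the kit otherwise stays in the world.
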(event `self.ReceiveBeginPlay`
  (bind _asbp_player (cast `/Game/Char/Player/BP_Player` (`GameplayStatics.GetPlayerCharacter` 0)))
  (set `self.PlayerRef` _asbp_player)
  (`self.FacingPlayer`))

(event `FacingPlayer`
  (bind (_returnvalue_roll _returnvalue_pitch _returnvalue_yaw) (`KismetMathLibrary.BreakRotator` (`KismetMathLibrary.RInterpTo` (`self.K2_GetActorRotation`) (`KismetMathLibrary.FindLookAtRotation` (`self.K2_GetActorLocation`) (`self.K2_GetActorLocation` (`self.PlayerRef`))) (`GameplayStatics.GetWorldDeltaSeconds`) 150.0)))
  (`self.K2_SetActorRotation` (`KismetMathLibrary.MakeRotator` 0.0 0.0 _returnvalue_yaw) :!label _label)
  (`KismetSystemLibrary.RetriggerableDelay` 0.2)
  (goto _label))

(event `self.MedKitCollider.OnComponentBeginOverlap`
  (params (OverlappedComponent :type "PrimitiveComponent Object Reference") (OtherActor :type "Actor Object Reference") (OtherComp :type "PrimitiveComponent Object Reference") (OtherBodyIndex :type Integer) (bFromSweep :type Boolean) (SweepResult :type "HitResult Structure (by ref)"))
  (bind _asbp_player (cast `/Game/Char/Player/BP_Player` OtherActor))
  (if (not (>= (`/Game/Char/Player/BP_Player.CurrentHealth` _asbp_player) (`/Game/Char/Player/BP_Player.MaxHealth` _asbp_player)))
    (`/Game/Char/Player/BP_Player.Add Health` _asbp_player 20.0)
    (`self.K2_DestroyActor`)))

(fn `UserConstructionScript`)
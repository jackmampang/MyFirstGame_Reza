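; Enemy spawner actor that populates the surrounding navigable area with BP_Enemy instances, up to MaxEnemyCount.
; SpawnEnemy starts a looping timer whose random interval is rolled once; each tick spawns at a random reachable point around the actor and increments EnemyCounter.
; The counter never decreases here, so the cap limits total spawns.
; BeginPlay and SpawnEnemybyPlayer are empty, so spawning relies on an external SpawnEnemy call.
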(event `self.ReceiveBeginPlay`)

(event `/Game/Char/BP_SystemInterface.SpawnEnemy`
  (`KismetSystemLibrary.K2_SetTimerDelegate` (delegate `SpawnTime`) (`KismetMathLibrary.RandomFloatInRange` 1.0 3.0) true))

(event `/Game/Char/BP_SystemInterface.SpawnEnemyByPlayer`)

(event `SpawnTime`
  (if (< (`self.EnemyCounter`) (`self.MaxEnemyCount`))
    (`|SpawnActorFromClass` "/Game/Char/Enemy/BP_Enemy.BP_Enemy_C" (`KismetMathLibrary.MakeTransform` (`NavigationSystemV1.K2_GetRandomReachablePointInRadius` (`self.K2_GetActorLocation`) 5000.0 null null) (`self.K2_GetActorRotation`)) "Undefined" "MultiplyWithRoot" null null)
    (set `self.EnemyCounter` (+ (`self.EnemyCounter`) 1))))

(fn `UserConstructionScript`)
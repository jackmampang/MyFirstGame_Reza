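; Rifle enemy that chases and shoots the player, driven by Blueprint events and AIMoveTo.
; Pawn sensing or taking damage starts a chase leading into montage-driven line-trace fire with reloads; player death switches it to random patrol.
; Damage flashes an outline and updates health; death plays animation, then a timeline-driven material dissolve handles score, random drops and destruction.
; Knockback blocks damage and firing, while exploder overlap triggers a physics impulse.
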(event `self.ReceiveTick`
  (params (DeltaSeconds :type "Float (single-precision)"))
  ;[1 1 1] EventTick
  (`/Engine/EditorBlueprintResources/StandardMacros.IsValid` (`self.WBP Health Bar`)
    (:`Is Valid`
      (`/Game/Char/Player/WBP_HealthBar.Set Health Bar` (`self.WBP Health Bar`) (`self.CurrentHealth`) (`self.MaxHealth`))
      (`SceneComponent.K2_SetWorldRotation` (`self.HeatlhBar`) (`KismetMathLibrary.FindLookAtRotation` (`self.K2_GetActorLocation`) (`self.K2_GetActorLocation` (`GameplayStatics.GetPlayerCameraManager` 0))) false false))))

(event `self.ReceiveBeginPlay`
  ;[1 1 1] BeginPlay
  (bind _asbp_player (cast `/Game/Char/Player/BP_Player` (`GameplayStatics.GetPlayerCharacter` 0)))
  (set `self.PlayerRef` _asbp_player)
  (bind _aswbp_health_bar (cast `/Game/Char/Player/WBP_HealthBar` (`WidgetComponent.GetWidget` (`self.HeatlhBar`))))
  (set `self.WBP Health Bar` _aswbp_health_bar))

(event `SpawnDrops`
  ;[1 1 1] SpawnDrops
  (`|SpawnActorFromClass` (select `int` (`KismetMathLibrary.RandomInteger` 3) :`0` "/Game/Char/Trinkets/BP_AmmoKit.BP_AmmoKit_C" :`1` "/Game/Char/Trinkets/BP_MedKit.BP_MedKit_C" :`2` null :!type "Actor Class Reference") (`KismetMathLibrary.MakeTransform` (`self.K2_GetActorLocation`)) "Undefined" "MultiplyWithRoot" null null))

(event `self.ReceiveAnyDamage`
  (params (Damage :type "Float (single-precision)") (DamageType :type "DamageType Object Reference") (InstigatedBy :type "Controller Object Reference") (DamageCauser :type "Actor Object Reference"))
  ;[1 1 1] AnyDamage
  (if (not (`self.IsDead`))
    (if (not (`self.IsKnocked`))
      (`self.ChasePlayer` DamageCauser)
      (`MeshComponent.SetOverlayMaterial` (`self.Mesh`) "/Game/Char/Player/Rory/MI_EnemyOutline.MI_EnemyOutline")
      (`KismetSystemLibrary.Delay` 1.0)
      (`MeshComponent.SetOverlayMaterial` (`self.Mesh`) null)
      (bind _output_get (set `self.CurrentHealth` (- (`self.CurrentHealth`) Damage)))
      (`KismetSystemLibrary.PrintString` (`KismetStringLibrary.Conv_DoubleToString` _output_get))
      (`self.UpdateHealthBar`)
      (if (<= (`self.CurrentHealth`) 0.0)
        (set `self.IsDead` true)
        (if (`self.IsKnocked`)
          (`SkeletalMeshComponent.PlayAnimation` (`self.Mesh`) "/Game/Char/Animation/SweepFall_UE.SweepFall_UE" false)
          (else
            (`SkeletalMeshComponent.PlayAnimation` (`self.Mesh`) (select `int` (`KismetMathLibrary.RandomInteger` 2) :`0` "/Game/Char/Animation/death_01.death_01" :`1` "/Game/Char/Animation/death_02.death_02" :!type "AnimationAsset Object Reference") false)
            (`KismetSystemLibrary.Delay` 0.5)
            (`SceneComponent.SetVisibility` (`self.HealthBarWidget`) false false)
            (`self.DissolveDeath`)))
        (elif (`self.IsKnocked`)
          (`|PlayMontage` (`self.Mesh`) "/Game/Char/Animation/AM_SweepFall.AM_SweepFall"
            (:`OnCompleted`
              _)
            (:`OnBlendOut`
              _))
          (bind _returnvalue (`self.PlayAnimMontage` "/Game/Char/Animation/AM_StandUp1.AM_StandUp1"))
          (`KismetSystemLibrary.Delay` _returnvalue)
          (set `self.IsKnocked` false))))))

(event `Patrol`
  ;[1 1 1] Patrol
  (set `self.IsChasing` false)
  (set `CharacterMovementComponent.MaxWalkSpeed` 300.0 (`self.CharacterMovement`))
  (`|AIMoveTo` self (`NavigationSystemV1.K2_GetRandomReachablePointInRadius` (`self.K2_GetActorLocation`) 5000.0 null null) null 50.0))

(event `/Game/Char/BP_SystemInterface.EnemyKnockBack`
  ;[1 1 1] KnockBack
  (if (not (`self.IsDead`))
    (set `self.IsKnocked` true)
    (`KismetSystemLibrary.Delay` 0.2)))

(event `DissolveDeath`
  ;[1 0 0.3128] DissolveDeath
  (`PrimitiveComponent.SetCollisionEnabled` (`self.CapsuleComponent`) "NoCollision")
  (`KismetSystemLibrary.Delay` 1.0)
  (bind _returnvalue (`PrimitiveComponent.CreateDynamicMaterialInstance` (`self.Mesh`) 0 "/Game/Char/Enemy/MI_Enemy.MI_Enemy" "None"))
  (bind _output_get (set `self.DeadMaterial` _returnvalue))
  (bind (_direction _dissolvetrack) (`Timeline|Timeline` :!via `PlayFromStart`)
    (:`Update`
      (`MaterialInstanceDynamic.SetScalarParameterValue` _output_get "Dissolve" (`KismetMathLibrary.Lerp` 0.0 1.0 _dissolvetrack))
      (`self.AddScore`)
      (`self.SpawnDrops`)
      (`self.K2_DestroyActor`))))

(event `/Game/Char/BP_SystemInterface.AIToggle`
  ;[1 1 1] AIToggle
  (`/Engine/EditorBlueprintResources/StandardMacros.FlipFlop`
    (:`A`
      (set `self.IsPawnSensing` true))
    (:`B`
      (set `self.IsPawnSensing` false))))

(event `AddScore`
  (bind _playerref (`self.PlayerRef`))
  ;[1 1 1] AddScore
  (set `/Game/Char/Player/BP_Player.Score` (+ (`/Game/Char/Player/BP_Player.Score` _playerref) (`self.ScorePoint`)) _playerref))

(event `self.PawnSensing.OnSeePawn`
  (params (Pawn :type "Pawn Object Reference"))
  ;[1 1 1] PawnSensing
  (if (not (`self.IsDead`))
    (`|ExecutionSequence`
      (:`then_0`
        (`self.ChasePlayer` (`GameplayStatics.GetPlayerCharacter` 0)))
      (:`then_1`
        (`self.Fire`)))))

(event `/Game/Char/BP_SystemInterface.Ragdoll`
  ;[1 1 1] Ragdoll
)

(event `ChasePlayer`
  (params (TargetActor :type "Actor Object Reference"))
  (bind (_returnvalue_roll _returnvalue_pitch _returnvalue_yaw) (`KismetMathLibrary.BreakRotator` (`KismetMathLibrary.FindLookAtRotation` (`self.K2_GetActorLocation`) (`self.K2_GetActorLocation` (`GameplayStatics.GetPlayerCharacter` 0)))))
  ;[1 1 1] ChasePlayer
  (set `self.IsChasing` true)
  (if (`self.IsDead`)
    _
    (elif (`self.IsKnocked`)
      _
      (elif (not (`/Game/Char/Player/BP_Player.IsDead` (`self.PlayerRef`)))
        (set `CharacterMovementComponent.MaxWalkSpeed` 450.0 (`self.CharacterMovement`))
        (`|AIMoveTo` self (`self.K2_GetActorLocation` (`self.PlayerRef`)) TargetActor (`KismetMathLibrary.RandomFloatInRange` 300.0 500.0)
          (:`OnSuccess`
            _)
          (:`OnFail`
            _))
        (`self.K2_SetActorRotation` (`KismetMathLibrary.MakeRotator` 0.0 0.0 _returnvalue_yaw))
        (`self.Fire`)))))

(event `self.Box.OnComponentBeginOverlap`
  (params (OverlappedComponent :type "PrimitiveComponent Object Reference") (OtherActor :type "Actor Object Reference") (OtherComp :type "PrimitiveComponent Object Reference") (OtherBodyIndex :type Integer) (bFromSweep :type Boolean) (SweepResult :type "HitResult Structure (by ref)"))
  (bind _asbp_exploder (cast `/Game/Char/Player/BP_Exploder` OtherActor))
  (set `self.Exploder ColliderRef` (`/Game/Char/Player/BP_Exploder.ExploderCollider` _asbp_exploder))
  (`PrimitiveComponent.SetSimulatePhysics` (`self.Mesh`) true)
  (`PrimitiveComponent.AddImpulseAtLocation` (`self.Mesh`) (`KismetMathLibrary.GetForwardVector` (`self.K2_GetActorRotation` (`self.PlayerRef`))) (`KismetMathLibrary.GetForwardVector` (`self.K2_GetActorRotation`)) "None"))

(event `Fire`
  (bind _returnvalue (`SceneComponent.GetSocketLocation` (`self.EnemyGun`) "MuzzleSocket"))
  ;[1 1 1] Fire
  (if (>= (`self.CurrentAmmo`) 1)
    (if (not (`self.IsKnocked`))
      (`|ExecutionSequence`
        (:`then_0`
          (`/Engine/EditorBlueprintResources/StandardMacros.DoOnce` false :!label _label
            (:`Completed`
              (`|PlayMontage` (`self.Mesh`) "/Game/Char/Animation/AM_FireRiffleIronSight.AM_FireRiffleIronSight"
                (:`then`
                  (bind _output_get (set `self.CurrentAmmo` (`KismetMathLibrary.Clamp` (- (`self.CurrentAmmo`) 1) 0 10)))
                  (if (== _output_get 0)
                    (`KismetSystemLibrary.Delay` 0.5)
                    (`self.Reload`)
                    (else
                      (bind (_outhit _returnvalue_2) (`KismetSystemLibrary.LineTraceSingle` :`Start` _returnvalue :`End` (+ _returnvalue (* (`SceneComponent.GetRightVector` (`self.Mesh`)) 600.0)) :`TraceChannel` "TraceTypeQuery1" :`DrawDebugType` "ForDuration"))
                      (if _returnvalue_2
                        (bind _asbp_player (cast `/Game/Char/Player/BP_Player` (`.HitActor` (`GameplayStatics.BreakHitResult` _outhit))))
                        (`GameplayStatics.ApplyDamage` _asbp_player 5.0 null null "/Script/Engine.DamageType")))))))))
        (:`then_1`
          (`KismetSystemLibrary.Delay` 0.4)
          (goto _label :!via `Reset`))))))

(event `PlayerIsDead`
  (`self.Patrol` self))

(event `Reload`
  ;[1 1 1] Reload
  (`|PlayMontage` (`self.Mesh`) "/Game/Char/Animation/AM_Reload.AM_Reload"
    (:`OnCompleted`
      (set `self.CurrentAmmo` 10)
      (`self.ChasePlayer` (`self.PlayerRef`)))))

(event `HealthBar`
  (bind _healthbarwidget (`self.HealthBarWidget`))
  ;[1 1 1] HealthBar
  (`SceneComponent.K2_SetWorldRotation` _healthbarwidget (`KismetMathLibrary.FindLookAtRotation` (`SceneComponent.K2_GetComponentLocation` _healthbarwidget) (`SceneComponent.K2_GetComponentLocation` (`PlayerCameraManager.TransformComponent` (`GameplayStatics.GetPlayerCameraManager` 0)))) false false :!label _label_2)
  (`KismetSystemLibrary.RetriggerableDelay` 0.2)
  (goto _label_2))

(fn `UpdateHealthBar`
  (bind _asbp_ui_enemy (cast `/Game/Char/Enemy/BP_UI_Enemy` (`WidgetComponent.GetUserWidgetObject` (`self.HealthBarWidget`))))
  (set `/Game/Char/Enemy/BP_UI_Enemy.HealthUI` (`self.CurrentHealth`) _asbp_ui_enemy)
  (return))

(fn `UserConstructionScript`)